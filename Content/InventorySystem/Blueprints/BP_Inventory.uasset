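; Slot-based player inventory that stores item classes with amounts and creates the main inventory widget on BeginPlay.
; Adding items recursively fills partial stacks then empty slots up to MaxStackSize, returning any remainder and optionally queuing an obtained-item message.
; Slots support remove, swap, split and merge, refreshing their slot widgets after changes.
; Using an item spawns its class as an actor and calls its OnUsed event.
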(event Custom|UpdateSlotAtIndex
  (params (Index :type Integer))
  (Default|UpdateSlot (Utilities|Array|Get(acopy) (Variables|/Game/InventorySystem/Widgets/WBP_Inventory.WBP_Inventory_C|GetSlotsWidgets (Variables|Default|GetInventory%20Widget%20Ref)) Index)))

(event Custom|UseItemAtIndex
  (params (Index :type Integer))
  (bind _slots (Variables|Default|GetSlots))
  (bind _output (Utilities|Array|Get(acopy) _slots Index))
  (if (Utilities|IsValidClass (.itemclass _output))
    (bind _returnvalue (Game|SpawnActorfromClass (.itemclass _output) (Math|Transform|MakeTransform "0, 0, 0" "0, 0, 0" "1,1,1") "AlwaysSpawn" 0 self Index 0))
    (Default|EventonUsed _returnvalue)))

(event EventBeginPlay
  (Utilities|Array|Resize (Variables|Default|GetSlots) (Variables|Default|GetAmountOfSlots))
  (bind _returnvalue (UserInterface|CreateWidget "/Game/InventorySystem/Widgets/WBP_MainWidget.WBP_MainWidget_C" (Game|GetPlayerController 0) self (Variables|Default|GetSlots%20Per%20Row) (Variables|Default|GetObtained%20Visible%20Timer)))
  (bind _output_get (Variables|Default|SetMain%20Widget%20Ref _returnvalue))
  (Variables|Default|SetInventory%20Widget%20Ref (Variables|/Game/InventorySystem/Widgets/WBP_MainWidget.WBP_MainWidget_C|GetInventoryWidget _output_get))
  (UserInterface|Viewport|AddtoViewport (Variables|Default|GetMain%20Widget%20Ref) 0)
  (if (not (Variables|Default|GetShow%20Obtained%20Message%20?))
    (Widget|RemovefromParent (Variables|/Game/InventorySystem/Widgets/WBP_MainWidget.WBP_MainWidget_C|GetObtainedItemBorder (Variables|Default|GetMain%20Widget%20Ref)))))

(fn ConstructionScript)

(fn IsSlotEmpty?
  (params (Index :type Integer))
  (return (not (Utilities|IsValidClass (.itemclass (Utilities|Array|Get(acopy) (Variables|Default|GetSlots) Index))))))

(fn GetItemInfoatIndex
  (params (Index :type Integer))
  (bind _slots (Variables|Default|GetSlots))
  (bind _output (Utilities|Array|Get(acopy) _slots Index))
  (return (not (Utilities|IsValidClass (.itemclass _output))) (.ItemInfo (Utilities|GetClassDefaults (.itemclass _output))) (.amount _output)))

(fn SearchEmptySlot
  (bind (_array_element _array_index) (Utilities|Array|ForEachLoopwithBreak (Variables|Default|GetSlots))
    (:LoopBody
      (if (not (Utilities|IsValidClass (.ItemClass (Utilities|Struct|BreakS_InventorySlot _array_element))))
        (return true _array_index)))
    (:Completed
      (return false -1))))

(fn SearchFreeStack
  (params (Item%20Class :type BP%20Master%20Item%20Class%20Reference))
  (bind (_array_element _array_index) (Utilities|Array|ForEachLoopwithBreak (Variables|Default|GetSlots))
    (:LoopBody
      (if (Math|Boolean|ANDBoolean (Utilities|IsValidClass (.ItemClass (Utilities|Struct|BreakS_InventorySlot _array_element))) (== Item%20Class (.ItemClass (Utilities|Struct|BreakS_InventorySlot _array_element))) (< (.Amount (Utilities|Struct|BreakS_InventorySlot _array_element)) (Variables|Default|GetMaxStackSize)))
        (return true _array_index)))
    (:Completed
      (return false -1))))

(fn AddItem
  (params (Item%20Class :type BP%20Master%20Item%20Class%20Reference) (Amount :type Integer))
  (if (Variables|Default|GetShow%20Obtained%20Message%20?)
    (bind (_success___ _rest_) (CallFunction|AddItem(Internal) Item%20Class Amount))
    (if _success___
      (CallFunction|ShowObtainedItem Item%20Class Amount)
      (return true _rest_)
      (else
        (return false _rest_)))
    (else
      (bind (_success____2 _rest__2) (CallFunction|AddItem(Internal) Item%20Class Amount))
      (return _success____2 _rest__2))))

(fn GetAmountatIndex
  (params (Index :type Integer))
  (return (.amount (Utilities|Array|Get(acopy) (Variables|Default|GetSlots) Index))))

(fn ShowInventory
  (bind _inventory_widget_ref (Variables|Default|GetInventory%20Widget%20Ref))
  (Widget|SetVisibility _inventory_widget_ref "Visible")
  (Widget|SetIsEnabled _inventory_widget_ref true)
  (Variables|Default|SetIs%20Visible%20? true))

(fn HideInventory
  (bind _inventory_widget_ref (Variables|Default|GetInventory%20Widget%20Ref))
  (Widget|SetVisibility _inventory_widget_ref "Hidden")
  (Widget|SetIsEnabled _inventory_widget_ref false)
  (Variables|Default|SetIs%20Visible%20? false)
  (Class|WidgetBlueprintLibrary|SetFocustoGameViewport)
  (Widget|SetIsEnabled (Variables|Default|GetInventory%20Widget%20Ref) false)
  (Widget|SetVisibility (Variables|/Game/InventorySystem/Widgets/WBP_MainWidget.WBP_MainWidget_C|GetThrowWidget (Variables|Default|GetMain%20Widget%20Ref)) "Hidden")
  (Widget|SetIsEnabled (Variables|/Game/InventorySystem/Widgets/WBP_Inventory.WBP_Inventory_C|GetSlotPanel (Variables|Default|GetInventory%20Widget%20Ref)) true))

(fn RemoveItematIndex
  (params (Index :type Integer) (Amount :type Integer))
  (bind _slots (Variables|Default|GetSlots))
  (bind _output (Utilities|Array|Get(acopy) _slots Index))
  (if (== Amount 0)
    (return true)
    (else
      (bind _empty__ (CallFunction|IsSlotEmpty? Index))
      (if _empty__
        (return false)
        (else
          (bind _amount (CallFunction|GetAmountatIndex Index))
          (if (>= Amount _amount)
            (Utilities|Array|SetArrayElem (Variables|Default|GetSlots) Index (Utilities|Struct|MakeS_InventorySlot 0 0))
            (else
              (Utilities|Array|SetArrayElem _slots Index (Utilities|Struct|MakeS_InventorySlot (.itemclass _output) (- (.amount _output) Amount)))))
          (CallFunction|UpdateSlotatIndex Index)
          (return true))))))

(fn SwapSlots
  (params (Index%201 :type Integer) (Index%202 :type Integer))
  (bind _slots (Variables|Default|GetSlots))
  (bind _slots_2 (Variables|Default|GetSlots))
  (bind _returnvalue (Utilities|Array|LastIndex _slots_2))
  (if (== Index%201 Index%202)
    (return true)
    (elif (and (<= Index%201 _returnvalue) (<= Index%202 _returnvalue))
      (LocalVariables|SetIndex%201%20Tmp (Utilities|Array|Get(acopy) _slots Index%201))
      (Utilities|Array|SetArrayElem _slots Index%201 (Utilities|Array|Get(acopy) _slots Index%202))
      (CallFunction|UpdateSlotatIndex Index%201)
      (Utilities|Array|SetArrayElem _slots Index%202 (LocalVariables|GetIndex%201%20Tmp))
      (CallFunction|UpdateSlotatIndex Index%202)
      (return true)
      (else
        (return false)))))

(fn SplitStack
  (params (Index :type Integer))
  (bind _slots (Variables|Default|GetSlots))
  (bind _output (Utilities|Array|Get(acopy) _slots Index))
  (bind _empty__ (CallFunction|IsSlotEmpty? Index))
  (if _empty__
    (return false)
    (else
      (bind _amount (CallFunction|GetItemInfoatIndex Index))
      (LocalVariables|SetAmount%20At%20Index _amount)
      (bind (_success__ _index) (CallFunction|SearchEmptySlot))
      (if _success__
        (LocalVariables|SetNew%20Amount (- (LocalVariables|GetAmount%20At%20Index) (/ (LocalVariables|GetAmount%20At%20Index) 2)))
        (Utilities|Array|SetArrayElem (Variables|Default|GetSlots) Index (Utilities|Struct|MakeS_InventorySlot (.itemclass _output) (- (LocalVariables|GetAmount%20At%20Index) (LocalVariables|GetNew%20Amount))))
        (CallFunction|UpdateSlotatIndex Index)
        (Utilities|Array|SetArrayElem (Variables|Default|GetSlots) _index (Utilities|Struct|MakeS_InventorySlot (.itemclass _output) (LocalVariables|GetNew%20Amount)))
        (CallFunction|UpdateSlotatIndex _index)
        (return true)
        (else
          (return false))))))

(fn TransferItemtoIndex
  (params (From%20Index :type Integer) (To%20Index :type Integer))
  (bind _slots (Variables|Default|GetSlots))
  (bind _slots_2 (Variables|Default|GetSlots))
  (bind _slots_3 (Variables|Default|GetSlots))
  (bind _output (Utilities|Array|Get(acopy) _slots_3 To%20Index))
  (bind _output_2 (Utilities|Array|Get(acopy) _slots To%20Index))
  (bind _output_3 (Utilities|Array|Get(acopy) _slots_3 From%20Index))
  (bind _output_4 (Utilities|Array|Get(acopy) _slots_2 To%20Index))
  ;[1 1 1] Are those 2 items the same ?
  ; Does the destination slot still have space ?
  ; Is the item stackable ?
  (bind _item_info (CallFunction|GetItemInfoatIndex To%20Index))
  (if (Math|Boolean|ANDBoolean (== (.itemclass (Utilities|Array|Get(acopy) (Variables|Default|GetSlots) From%20Index)) (.itemclass _output_2)) (< (.amount _output_2) (Variables|Default|GetMaxStackSize)) (.IsStackable? (Utilities|Struct|BreakS_ItemInfo _item_info)))
    ;[1 1 1] Yes, will the transfer overflow the slot ?
    (if (> (+ (.amount (Utilities|Array|Get(acopy) (Variables|Default|GetSlots) From%20Index)) (.amount (Utilities|Array|Get(acopy) (Variables|Default|GetSlots) To%20Index))) (Variables|Default|GetMaxStackSize))
      ;[1 1 1] Yes, (Addition of both) - Max Stack for the base, Max Stack Size for the destination
      (Utilities|Array|SetArrayElem _slots_3 From%20Index (Utilities|Struct|MakeS_InventorySlot (.itemclass _output_3) (- (+ (.amount _output_3) (.amount _output)) (Variables|Default|GetMaxStackSize))))
      (Utilities|Array|SetArrayElem (Variables|Default|GetSlots) To%20Index (Utilities|Struct|MakeS_InventorySlot (.itemclass _output) (Variables|Default|GetMaxStackSize)))
      (else
        ;[1 1 1] No, make the addition and remove base Slot
        (Utilities|Array|SetArrayElem _slots_2 To%20Index (Utilities|Struct|MakeS_InventorySlot (.itemclass _output_4) (+ (.amount (Utilities|Array|Get(acopy) _slots_2 From%20Index)) (.amount _output_4))))
        (Utilities|Array|SetArrayElem (Variables|Default|GetSlots) From%20Index (Utilities|Struct|MakeS_InventorySlot 0 0))))
    (CallFunction|UpdateSlotatIndex From%20Index)
    (CallFunction|UpdateSlotatIndex To%20Index)
    (return true)
    (else
      ;[1 1 1] No, failure
      (return false))))

(fn ShowObtainedItem
  (params (Item%20Class :type BP%20Master%20Item%20Class%20Reference) (Amount :type Integer))
  (bind _main_widget_ref (Variables|Default|GetMain%20Widget%20Ref))
  (if (Variables|Default|GetShow%20Obtained%20Message%20?)
    (Utilities|IsValid _main_widget_ref
      (:Is%20Valid
        (Default|AddItemtoObtainedQueue _main_widget_ref Item%20Class Amount)
        (return true))
      (:Is%20Not%20Valid
        _)))
  (return false))

(fn AddItem(Internal)
  (params (Item%20Class :type BP%20Master%20Item%20Class%20Reference) (Amount :type Integer))
  (bind _slots (Variables|Default|GetSlots))
  ;[1 1 1] Does the Class exist ?
  (if (Utilities|IsValidClass Item%20Class)
    ;[1 1 1] Is the Item Stackable ?
    (if (.IsStackable? (Utilities|Struct|BreakS_ItemInfo (.ItemInfo (Utilities|GetClassDefaults Item%20Class))))
      ;[1 1 1] Stackable ? Ok, is there any free usuable stacks in the Inventory ?
      (bind (_success__ _index) (CallFunction|SearchFreeStack Item%20Class))
      (if _success__
        ;[1 1 1] Yes ? Ok, will the current amount overflow the current stack ?
        (if (> (+ (.amount (Utilities|Array|Get(acopy) (Variables|Default|GetSlots) _index)) Amount) (Variables|Default|GetMaxStackSize))
          ;[1 1 1] Yes, set the max size amount to the current Slot and recursive call
          (LocalVariables|SetOverflow (- (+ (.amount (Utilities|Array|Get(acopy) (Variables|Default|GetSlots) _index)) Amount) (Variables|Default|GetMaxStackSize)))
          (Utilities|Array|SetArrayElem _slots _index (Utilities|Struct|MakeS_InventorySlot Item%20Class (Variables|Default|GetMaxStackSize)))
          (CallFunction|UpdateSlotatIndex _index)
          (bind _rest_ (CallFunction|AddItem(Internal) Item%20Class (LocalVariables|GetOverflow)))
          (return true _rest_)
          (else
            ;[1 1 1] No, add it
            (Utilities|Array|SetArrayElem _slots _index (Utilities|Struct|MakeS_InventorySlot Item%20Class (+ (.amount (Utilities|Array|Get(acopy) (Variables|Default|GetSlots) _index)) Amount)))
            (CallFunction|UpdateSlotatIndex _index)
            (return true 0)))
        (else
          ;[1 1 1] No ? Ok, try to find an empty slot for the current stack then (recursive call if stack > Max Stack Size)
          (bind (_success___2 _index_2) (CallFunction|SearchEmptySlot))
          (if _success___2
            (if (> Amount (Variables|Default|GetMaxStackSize))
              (Utilities|Array|SetArrayElem (Variables|Default|GetSlots) _index_2 (Utilities|Struct|MakeS_InventorySlot Item%20Class (Variables|Default|GetMaxStackSize)))
              (CallFunction|UpdateSlotatIndex _index_2)
              (bind _rest__2 (CallFunction|AddItem(Internal) Item%20Class (- Amount (Variables|Default|GetMaxStackSize))))
              (return true _rest__2)
              (else
                (Utilities|Array|SetArrayElem (Variables|Default|GetSlots) _index_2 (Utilities|Struct|MakeS_InventorySlot Item%20Class Amount))
                (CallFunction|UpdateSlotatIndex _index_2)
                (return true 0)))
            (else
              (return true Amount)))))
      (else
        ;[1 1 1] Not Stackable ? Ok, try to find an empty slot and add the item (recursive call if > 1 amount)
        (bind (_success___3 _index_3) (CallFunction|SearchEmptySlot))
        (if _success___3
          (Utilities|Array|SetArrayElem (Variables|Default|GetSlots) _index_3 (Utilities|Struct|MakeS_InventorySlot Item%20Class 1))
          (CallFunction|UpdateSlotatIndex _index_3)
          (if (> Amount 1)
            (bind _rest__3 (CallFunction|AddItem(Internal) Item%20Class (- Amount 1)))
            (return true _rest__3)
            (else
              (return true 0)))
          (else
            (return true Amount)))))
    (else
      (return false Amount))))