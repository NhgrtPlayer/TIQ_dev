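; BP_PickUpItem is a world pickup that adds an item to the side-scroller character's inventory on contact.
; When a SideScrollerCharacter overlaps PickUpRadius, it passes ItemToAdd and AmountToAdd to AddItem on the character's InventoryRef, if valid.
; On success, any leftover amount stays in the pickup as the new AmountToAdd, otherwise the actor destroys itself.
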(event OnComponentBeginOverlap(PickUpRadius)
  (params (OverlappedComponent :type Primitive%20Component%20Object%20Reference) (OtherActor :type Actor%20Object%20Reference) (OtherComp :type Primitive%20Component%20Object%20Reference) (OtherBodyIndex :type Integer) (bFromSweep :type Boolean) (SweepResult :type Hit%20Result%20Structure%20%28by%20ref%29))
  (bind _asside_scroller_character (Utilities|Casting|CastToSideScrollerCharacter OtherActor))
  (Utilities|IsValid (Variables|/Game/SideScrollerBP/Blueprints/SideScrollerCharacter.SideScrollerCharacter_C|GetInventoryRef _asside_scroller_character)
    (:Is%20Valid
      (bind (_success__ _rest) (Default|AddItem (Variables|/Game/SideScrollerBP/Blueprints/SideScrollerCharacter.SideScrollerCharacter_C|GetInventoryRef _asside_scroller_character) (Variables|Default|GetItemToAdd) (Variables|Default|GetAmountToAdd)))
      (if _success__
        (if (> _rest 0)
          (Variables|Default|SetAmountToAdd _rest)
          (else
            (Actor|DestroyActor)))))))

(event EventBeginPlay)

(event Collision|EventActorBeginOverlap
  (params (OtherActor :type Actor%20Object%20Reference)))

(event EventTick
  (params (DeltaSeconds :type Float%20%28single-precision%29)))

(fn ConstructionScript)