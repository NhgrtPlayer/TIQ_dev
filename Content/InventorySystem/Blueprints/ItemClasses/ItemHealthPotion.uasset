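; Health potion item for the inventory system that restores HP to the side-scroller character when used.
; The on-used event reaches the character through the inventory reference and, only if HP is below max, heals a fixed amount and removes one item at its stored index.
; The item actor destroys itself after use, whether or not the heal happens.
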(event EventBeginPlay
  (|CallParentFunction))

(event Collision|EventActorBeginOverlap
  (params (OtherActor :type Actor%20Object%20Reference))
  (|CallParentFunction OtherActor))

(event EventTick
  (params (DeltaSeconds :type Float%20%28single-precision%29))
  (|CallParentFunction DeltaSeconds))

(event EventEventonUsed
  (bind _inventory_ref (Variables|Default|GetInventory%20Ref))
  (bind _sidescrollercharref (Variables|/Game/InventorySystem/Blueprints/BP_Inventory.BP_Inventory_C|GetSideScrollerCharRef _inventory_ref))
  (if (< (Variables|/Game/SideScrollerBP/Blueprints/SideScrollerCharacter.SideScrollerCharacter_C|GetCurrent%20HP _sidescrollercharref) (Variables|/Game/SideScrollerBP/Blueprints/SideScrollerCharacter.SideScrollerCharacter_C|GetHP%20Max _sidescrollercharref))
    (Default|Heal _sidescrollercharref 100)
    (Default|RemoveItematIndex (Variables|Default|GetInventory%20Ref) (Variables|Default|GetIndex) 1))
  (Actor|DestroyActor))

(fn ConstructionScript
  (|CallParentFunction))