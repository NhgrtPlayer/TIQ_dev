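; ItemSword is an inventory item Blueprint for a sword that changes the side-scroller character's equipped weapon when used.
; On its used event, it reaches the character through the inventory reference and compares CurrentWeapon to ItemSword.
; A match calls EquipWeapon with ItemSword, while any other value calls UnequipWeapon.
; Tick and the construction script only call their parent versions.
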(event EventBeginPlay
  (|CallParentFunction) ; This node is disabled and will not be called.\nDrag off pins to build functionality.
)

(event Collision|EventActorBeginOverlap
  (params (OtherActor :type Actor%20Object%20Reference))
  (|CallParentFunction OtherActor) ; This node is disabled and will not be called.\nDrag off pins to build functionality.
)

(event EventEventonUsed
  (bind _inventory_ref (Variables|Default|GetInventory%20Ref))
  (bind _sidescrollercharref (Variables|/Game/InventorySystem/Blueprints/BP_Inventory.BP_Inventory_C|GetSideScrollerCharRef _inventory_ref))
  (if (== (Variables|/Game/SideScrollerBP/Blueprints/SideScrollerCharacter.SideScrollerCharacter_C|GetCurrent%20Weapon _sidescrollercharref) "ItemSword_C")
    (Default|EquipWeapon _sidescrollercharref "ItemSword_C")
    (else
      (Default|UnequipWeapon _sidescrollercharref))))

(event EventTick
  (params (DeltaSeconds :type Float%20%28single-precision%29))
  (|CallParentFunction DeltaSeconds))

(fn ConstructionScript
  (|CallParentFunction))